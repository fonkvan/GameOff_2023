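; Camera rail actor that travels along the level's BP_SplineRoute while panning its aim from Svarog to Gideon.
; Construction finds the spline and both characters (by SkeletalMeshActor array order), sets timeline rates from durations and snaps to the first point.
; On BeginPlay, MoveCamera drives position while TransitionBetweenPoints' playback position blends the two offset look-at rotations.
; Tick prints that playback position for debugging.
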(event `self.ReceiveBeginPlay`
  (bind _spline (`/Game/GameOff2023/Blueprints/LevelSelector/BP_SplineRoute.Spline` (`self.Spline`)))
  (`|ExecutionSequence`
    (:`then_0`
      (bind (_direction _newtrack_0) (`Timeline|MoveCamera`)
        (:`Update`
          (bind _angle (`self.GetRotatorToPoints` (+ (`self.K2_GetActorLocation` (`self.Svarog`)) (50.0 0.0 250.0)) (+ (`self.K2_GetActorLocation` (`self.Gideon`)) (100.0 0.0 200.0))))
          (`self.K2_SetActorTransform` (`KismetMathLibrary.MakeTransform` (`SplineComponent.GetLocationAtTime` (`/Game/GameOff2023/Blueprints/LevelSelector/BP_SplineRoute.Spline` (`self.Spline`)) (`KismetMathLibrary.Lerp` (`SplineComponent.GetTimeAtDistanceAlongSpline` _spline (`SplineComponent.GetDistanceAlongSplineAtSplinePoint` _spline 0)) (`SplineComponent.GetTimeAtDistanceAlongSpline` _spline (`SplineComponent.GetDistanceAlongSplineAtSplinePoint` _spline (- (`SplineComponent.GetNumberOfSplinePoints` _spline) 1))) _newtrack_0) "World" false) _angle)))))
    (:`then_1`
      (`Timeline|TransitionBetweenPoints`))))

(event `self.ReceiveTick`
  (params (DeltaSeconds :type "Float (single-precision)"))
  (`KismetSystemLibrary.PrintString` (`KismetStringLibrary.Conv_DoubleToString` (`TimelineComponent.GetPlaybackPosition` (`self.TransitionBetweenPoints`)))))

(fn `GetRotatorToPoints`
  (params (`Point 1` :type "Vector Structure") (`Point 2` :type "Vector Structure"))
  (returns (Angle :type "Rotator Structure"))
  (bind _returnvalue (`self.K2_GetActorLocation`))
  (return (`KismetMathLibrary.RLerp` (`KismetMathLibrary.FindLookAtRotation` _returnvalue `Point 1`) (`KismetMathLibrary.FindLookAtRotation` _returnvalue `Point 2`) (`TimelineComponent.GetPlaybackPosition` (`self.TransitionBetweenPoints`)))))

(fn `UserConstructionScript`
  (`|ExecutionSequence`
    (:`then_0`
      ;[1 1 1] Init variables
      (`|ExecutionSequence`
        (:`then_0`
          (bind _returnvalue (`GameplayStatics.GetActorOfClass` "/Game/GameOff2023/Blueprints/LevelSelector/BP_SplineRoute.BP_SplineRoute_C"))
          (set `self.Spline` _returnvalue))
        (:`then_1`
          (bind _outactors (`GameplayStatics.GetAllActorsOfClass` "/Script/Engine.SkeletalMeshActor"))
          (for (_array_element _array_index) _outactors
            (switch `int` _array_index
              (:`0`
                (set `self.Gideon` _array_element))
              (:`1`
                (set `self.Svarog` _array_element)))))))
    (:`then_1`
      ;[1 1 1] Set time to traverse between watch points
      (`TimelineComponent.SetPlayRate` (`self.MoveCamera`) (/ 1.0 (`self.TimeToCompleteRoute`)))
      (`TimelineComponent.SetPlayRate` (`self.TransitionBetweenPoints`) (/ 1.0 (`self.TimeToCompleteTransition`))))
    (:`then_2`
      (`self.K2_SetActorLocation` (`SplineComponent.GetLocationAtSplinePoint` (`/Game/GameOff2023/Blueprints/LevelSelector/BP_SplineRoute.Spline` (`self.Spline`)) 0 "World")))))