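; Level selector spline actor that repeats a static mesh along a spline, built in the construction script.
; It takes segment length from the mesh bounds on a chosen axis plus UpScale, then adds spline mesh components to cover the spline length.
; Each segment deforms along X between sampled spline points, with offsets and a coefficient applied to positions and tangents clamped to segment length.
; The event graph is empty.
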(fn `UserConstructionScript`
  (bind _offsetcoefficient (`self.OffSetCoefficient`))
  (bind _offsetcoefficient_2 (`self.OffSetCoefficient`))
  (bind _spline (`self.Spline`))
  (bind _spline_2 (`self.Spline`))
  (bind (_returnvalue_min _returnvalue_max) (break `Box` (`StaticMesh.GetBoundingBox` (`self.Mesh`))))
  (bind (_returnvalue_x _returnvalue_y _returnvalue_z) (`KismetMathLibrary.BreakVector` (+ (`KismetMathLibrary.Vector_GetAbs` _returnvalue_min) (`KismetMathLibrary.Vector_GetAbs` _returnvalue_max))))
  (switch `/Game/GameOff2023/Blueprints/LevelSelector/SplineLengthAxis` (`self.LengthAxis`)
    (:`NewEnumerator0`
      (set `self.Length` _returnvalue_x))
    (:`NewEnumerator1`
      (set `self.Length` _returnvalue_y))
    (:`NewEnumerator2`
      (set `self.Length` _returnvalue_z)))
  (set `self.Length` (+ (`self.Length`) (`self.UpScale`)))
  (for _index (range (+ (`KismetMathLibrary.FTrunc` (/ (`SplineComponent.GetSplineLength` (`self.Spline`)) (`self.Length`))) 1))
    (bind _returnvalue (`AddComponent|NODE_AddSplineMeshComponent-0`))
    (`SplineMeshComponent.SetForwardAxis` _returnvalue "X" true)
    (`StaticMeshComponent.SetStaticMesh` _returnvalue (`self.Mesh`))
    (bind _returnvalue_2 (* _index (`self.Length`)))
    (bind (_returnvalue_x_2 _returnvalue_y_2 _returnvalue_z_2) (`KismetMathLibrary.BreakVector` (+ (`SplineComponent.GetLocationAtDistanceAlongSpline` _spline_2 _returnvalue_2 "Local") (`self.OffSetStart`))))
    (bind _returnvalue_3 (* (+ _index 1) (`self.Length`)))
    (bind (_returnvalue_x_3 _returnvalue_y_3 _returnvalue_z_3) (`KismetMathLibrary.BreakVector` (+ (`SplineComponent.GetLocationAtDistanceAlongSpline` _spline _returnvalue_3 "Local") (`self.OffSetStartEnd`))))
    (`SplineMeshComponent.SetStartAndEnd` _returnvalue (`KismetMathLibrary.MakeVector` (* _returnvalue_x_2 _offsetcoefficient_2) (* _returnvalue_y_2 _offsetcoefficient_2) (* _returnvalue_z_2 _offsetcoefficient_2)) (`KismetMathLibrary.ClampVectorSize` (`SplineComponent.GetTangentAtDistanceAlongSpline` _spline_2 _returnvalue_2 "Local") 0.0 (`self.Length`)) (`KismetMathLibrary.MakeVector` (* _returnvalue_x_3 _offsetcoefficient) (* _returnvalue_y_3 _offsetcoefficient) (* _returnvalue_z_3 _offsetcoefficient)) (`KismetMathLibrary.ClampVectorSize` (`SplineComponent.GetTangentAtDistanceAlongSpline` _spline _returnvalue_3 "Local") 0.0 (`self.Length`)) true)))